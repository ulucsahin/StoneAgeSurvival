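; BP_StoneAgeColonyCharacter is a character Blueprint that lets the player toggle an inventory screen with the I key.
; Opening creates a new PlayerInventory widget, adds it to the viewport, shows the mouse cursor and switches to game-and-UI input.
; Closing removes the widget, hides the cursor and restores game-only input, with the InventoryOn flag tracking state.
; A debug "Hello" prints on each press, and a cast to SurvivalPlayerController sits unconnected.
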(event Input|KeyboardEvents|I
  (params (Key :type Key%20Structure))
  (bind _returnvalue (Game|GetPlayerController 0))
  (bind _returnvalue_2 (Game|GetPlayerController 0))
  (:Pressed
    (Development|PrintString "Hello")
    (if (Variables|Default|GetInventoryOn)
      (Variables|/Script/Engine.PlayerController|SetbShowMouseCursor _returnvalue_2 false)
      (Input|SetInputModeGameOnly _returnvalue_2)
      (Widget|RemovefromParent (Variables|Default|GetInventoryWidget))
      (else
        (Variables|/Script/Engine.PlayerController|SetbShowMouseCursor _returnvalue true)
        (Input|SetInputModeGameandUI _returnvalue 0 "DoNotLock" false)
        (bind _returnvalue_3 (UserInterface|CreateWidget "/Game/Uluc/HUD/Inventory/PlayerInventory.PlayerInventory_C"))
        (bind _output_get (Variables|Default|SetInventoryWidget _returnvalue_3))
        (UserInterface|Viewport|AddtoViewport _output_get 0)))
    (Variables|Default|SetInventoryOn (not (Variables|Default|GetInventoryOn)))))

(fn ConstructionScript)